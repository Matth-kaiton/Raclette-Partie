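; BP_Spike is a spike trap that springs when the player pawn overlaps its trigger and kills the character it hits.
; The RevealSpike timeline moves the spike along relative Z, then a three-second delay and a DoOnce lead to the HideSpikes timeline, which moves it back and resets the DoOnce.
; A separate DeathBox overlap calls Death on any BP_ThirdPersonCharacter, with no check on the spike's state.
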(event OnComponentBeginOverlap(TrigerTrap)
  (params (OverlappedComponent :type Primitive%20Component%20Object%20Reference) (OtherActor :type Actor%20Object%20Reference) (OtherComp :type Primitive%20Component%20Object%20Reference) (OtherBodyIndex :type Integer) (bFromSweep :type Boolean) (SweepResult :type Hit%20Result%20Structure%20%28by%20ref%29))
  (if (== OtherActor (Game|Player|GetPlayerPawn 0))
    (CallFunction|SpikeStart)))

(event OnComponentBeginOverlap(DeathBox)
  (params (OverlappedComponent :type Primitive%20Component%20Object%20Reference) (OtherActor :type Actor%20Object%20Reference) (OtherComp :type Primitive%20Component%20Object%20Reference) (OtherBodyIndex :type Integer) (bFromSweep :type Boolean) (SweepResult :type Hit%20Result%20Structure%20%28by%20ref%29))
  (bind _asbp_third_person_character (Utilities|Casting|CastToBP_ThirdPersonCharacter OtherActor))
  (Default|Death _asbp_third_person_character))

(event Custom|Spike%20Start
  (bind _newtrack_0 (Timeline|Reveal%20Spike PlayFromStart)
    (:Update
      (Transformation|SetRelativeLocation (Variables|Default|Getspike) (Math|Vector|MakeVector 0.0 0.0 _newtrack_0) false false)
      (Utilities|FlowControl|Delay 3.0)
      (Utilities|FlowControl|DoOnce false
        (:Completed
          (CallFunction|SpikeEnd))))))

(event Custom|Spike%20End
  (bind _newtrack_0 (Timeline|hide%20spikes PlayFromStart)
    (:Update
      (Transformation|SetRelativeLocation (Variables|Default|Getspike) (Math|Vector|MakeVector 0.0 0.0 _newtrack_0) false false)
      (Utilities|FlowControl|DoOnce false) ; enters at Reset
    )))

(fn ConstructionScript)