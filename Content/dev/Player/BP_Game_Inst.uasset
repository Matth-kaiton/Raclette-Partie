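; BP_Game_Inst, apparently the game instance, holds the state of a random player malus.
; RandMalus clears the previous flags, then has a two-in-three chance to enable exactly one malus: pet, drunk ("Saoul") or inverted controls.
; ResetMalus clears all three flags, and debug prints show each roll and the chosen malus.
; The flags are only set here; their effects are not implemented in this graph.
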(event Custom|RandMalus
  (CallFunction|ResetMalus)
  (bind _output_get (Variables|Default|SetMalusChance (Math|Random|RandomInteger 3)))
  (Development|PrintString (Utilities|String|ToString(Integer) _output_get))
  (if (< 0 _output_get)
    (bind _output_get_2 (Variables|Default|Setmalus (Math|Random|RandomInteger 3)))
    (Development|PrintString (Utilities|String|ToString(Integer) _output_get_2))
    (switch int _output_get_2
      (:0
        (Development|PrintString "Pet")
        (Variables|Default|SetMalus_Pet true))
      (:1
        (Development|PrintString "Saoul")
        (Variables|Default|SetMalus_Saoul true))
      (:2
        (Development|PrintString "Controles")
        (Variables|Default|SetMalus_Invert_Controles true)))))

(event Custom|Reset%20Malus
  (Variables|Default|SetMalus_Pet false)
  (Variables|Default|SetMalus_Invert_Controles false)
  (Variables|Default|SetMalus_Saoul false))

(event Custom|begin)